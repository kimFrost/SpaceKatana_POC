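; BP_MovementField is an actor that shows a movement range as a flat procedural disc with radius MaxDistance.
; The construction script calls UpdateField, which builds a 200-segment triangle fan with collision, applies M_MovementField and draws debug points and edges.
; An unwired block would pull vertices inward near other movement fields.
; GetClosestValidLocation is an unfinished stub: it line-traces the mesh, loops with an empty body and never reaches its return.
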(fn `GetClosestValidLocation`
  (params (Location :type "Vector Structure"))
  (returns (ValidLocation :type "Vector Structure"))
  (bind (_hitlocation _hitnormal _bonename _returnvalue) (`PrimitiveComponent.K2_LineTraceComponent` (`self.ProceduralMesh`) (0.0 0.0 0.0) (0.0 0.0 0.0) true true))
  (if (not _returnvalue)
    (for _ (range (+ (`KismetMathLibrary.FCeil` (/ (`KismetMathLibrary.VSize` (- (`self.K2_GetActorLocation`) Location)) 0.1)) 1))
      _)))

(fn `UpdateField`
  (bind _returnvalue (`self.K2_GetActorLocation`))
  (bind _triangles (`self.Triangles`))
  (bind _proceduralmesh (`self.ProceduralMesh`))
  (bind _triangles_2 (`self.Triangles`))
  (bind _triangles_3 (`self.Triangles`))
  (bind _verticies (`self.Verticies`))
  (bind _returnvalue_2 (`KismetArrayLibrary.Array_LastIndex` (`self.Verticies`)))
  (`|ExecutionSequence`
    (:`then_0`
      (`KismetArrayLibrary.Array_Clear` (`self.Verticies`))
      (`KismetArrayLibrary.Array_Clear` (`self.Triangles`))
      ;[1 1 1] Center vertice
      (`KismetArrayLibrary.Array_Add` (`self.Verticies`) (0.0 0.0 0.0))
      (for _index (range 201)
        (`KismetArrayLibrary.Array_Add` (`self.Verticies`) (`KismetMathLibrary.RotateAngleAxis` (`KismetMathLibrary.MakeVector` (`self.MaxDistance`)) (* _index (/ 360.0 200.0)) (0.0 0.0 1.0)))
        (if (> _index 0)
          (`KismetArrayLibrary.Array_Add` _triangles_2)
          (`KismetArrayLibrary.Array_Add` _triangles_2 _index)
          (`KismetArrayLibrary.Array_Add` _triangles_2 (- _index 1))))
      (`KismetArrayLibrary.Array_Add` _triangles)
      (`KismetArrayLibrary.Array_Add` _triangles _returnvalue_2)
      (`KismetArrayLibrary.Array_Add` _triangles (- _returnvalue_2 1)))
    (:`then_1`)
    (:`then_2`
      (`ProceduralMeshComponent.ClearAllMeshSections` _proceduralmesh)
      (`ProceduralMeshComponent.CreateMeshSection_LinearColor` :`self` _proceduralmesh :`Vertices` (`self.Verticies`) :`Triangles` (`self.Triangles`) :`Normals` (`self.Normals`) :`UV0` (`self.UVs`) :`bCreateCollision` true)
      (`PrimitiveComponent.SetMaterial` (`self.ProceduralMesh`) 0 "/Game/SpaceKatana/Materials/M_MovementField.M_MovementField")
      ;[1 1 1] Debug
      (`|ExecutionSequence`
        (:`then_0`
          (for _array_element (`self.Verticies`)
            (`KismetSystemLibrary.DrawDebugPoint` (+ (`self.K2_GetActorLocation`) _array_element) 20.0 (struct :`R` 0.89 :`B` 0.821881 :`A` 1.0) 5.0)))
        (:`then_1`
          (for _index_2 (range (/ (`KismetArrayLibrary.Array_Length` (`self.Triangles`)) 3))
            (for _index_3 (range 3)
              (switch `int` _index_3
                (:`0`
                  (bind _returnvalue_3 (+ _index_3 (* _index_2 3)))
                  (bind _returnvalue_4 (+ _returnvalue (`KismetArrayLibrary.Array_Get` _verticies (`KismetArrayLibrary.Array_Get` _triangles_3 _returnvalue_3))))
                  (`KismetSystemLibrary.DrawDebugLine` _returnvalue_4 (+ _returnvalue (`KismetArrayLibrary.Array_Get` _verticies (`KismetArrayLibrary.Array_Get` _triangles_3 (+ _returnvalue_3 1)))) (struct :`R` 0.355765 :`G` 0.453407 :`B` 1.0 :`A` 1.0) 5.0 1.0 :!label _label))
                (:`1`
                  (goto _label))
                (:`2`
                  (`KismetSystemLibrary.DrawDebugLine` _returnvalue_4 (+ _returnvalue (`KismetArrayLibrary.Array_Get` _verticies (`KismetArrayLibrary.Array_Get` _triangles_3 (- _returnvalue_3 2)))) (struct :`R` 0.355765 :`G` 0.453407 :`B` 1.0 :`A` 1.0) 5.0 1.0))))))))))

(fn `UserConstructionScript`
  (`self.UpdateField`))