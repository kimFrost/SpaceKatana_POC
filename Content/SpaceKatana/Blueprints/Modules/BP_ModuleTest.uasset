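; BP_ModuleTest is a test module Blueprint that prints overlap information for debugging.
; On Tick, after the parent logic runs, it prints the display name of every actor overlapping its StaticMesh, refreshed each frame.
; BeginPlay and the construction script only call the parent, while a state-based print of the mesh's world location and several other overlap queries are left disconnected.
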(event `self.ReceiveBeginPlay`
  (`parent.ReceiveBeginPlay`))

(event `self.ReceiveTick`
  (params (DeltaSeconds :type "Float (single-precision)"))
  (`parent.ReceiveTick` DeltaSeconds)
  (for _array_element (`PrimitiveComponent.GetOverlappingActors` (`self.StaticMesh`) null)
    (`KismetSystemLibrary.PrintString` (`KismetSystemLibrary.GetDisplayName` _array_element) true true (struct :`G` 0.66 :`B` 1.0 :`A` 1.0) 0.0)))

(fn `UserConstructionScript`
  (`parent.UserConstructionScript`))