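; Space Katana weapon projectile that moves at a configurable speed, with a Lance type that acts as a short-lived hitscan laser.
; Lance disables collision and movement, line-traces forward, spawns BP_NovaHit at impact and stretches its mesh to that distance.
; Physical hits spawn BP_NovaHit, damage ships or destroy modules, then destroy the projectile.
; Tick draws a debug trail; UpdateMesh has no effect.
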(event `self.ReceiveTick`
  (params (DeltaSeconds :type "Float (single-precision)"))
  (bind _returnvalue (`self.K2_GetActorLocation`))
  (`KismetSystemLibrary.DrawDebugLine` _returnvalue (+ _returnvalue (* (`KismetMathLibrary.GreaterGreater_VectorRotator` (`self.GetActorForwardVector`) (struct :`Yaw` 180.0)) 30.0)) (struct :`R` 1.0 :`B` 0.697964 :`A` 1.0) 0.0 3.0))

(event `self.ReceiveBeginPlay`
  (bind _returnvalue (`self.K2_GetActorLocation`))
  (bind _staticmesh (`self.StaticMesh`))
  (switch `/Game/SpaceKatana/DATA/Enums/ProjectileType` (`self.Type`)
    (:`NewEnumerator3`
      (`StaticMeshComponent.SetStaticMesh` _staticmesh "/Game/SpaceKatana/Meshes/SM_ProjectileLance.SM_ProjectileLance")
      (`PrimitiveComponent.SetCollisionEnabled` (`self.StaticMesh`) "NoCollision")
      (set `ProjectileMovementComponent.InitialSpeed` 0.0 (`self.ProjectileMovement`))
      (`self.SetLifeSpan` 0.15)
      (`PrimitiveComponent.SetMaterial` _staticmesh 0 "/Game/SpaceKatana/Materials/Laser/M_Laser_Inst.M_Laser_Inst")
      ;[1 1 1] TraceHitWithLaser
      (bind (_outhit _returnvalue_2) (`KismetSystemLibrary.LineTraceSingle` :`Start` _returnvalue :`End` (+ _returnvalue (* (`self.GetActorForwardVector`) 5000.0)) :`TraceChannel` "TraceTypeQuery1" :`bTraceComplex` true :`DrawTime` 0.5))
      (if _returnvalue_2
        (bind (_bblockinghit _binitialoverlap _time _location) (`GameplayStatics.BreakHitResult` _outhit))
        (`|SpawnActorFromClass` "/Game/TwinStickBP/Blueprints/Actors/BP_NovaHit.BP_NovaHit_C" (`KismetMathLibrary.MakeTransform` _location) "Undefined" "OverrideRootScale" null (`self.DamagePower`))
        (`SceneComponent.SetRelativeScale3D` (`self.StaticMesh`) (`KismetMathLibrary.MakeVector` (/ (`KismetMathLibrary.VSize` (- (`self.K2_GetActorLocation`) _location)) 100.0) 1.0 1.0))
        (else
          (`SceneComponent.SetRelativeScale3D` (`self.StaticMesh`) (`KismetMathLibrary.MakeVector` 100.0 1.0 1.0)))))))

(event `self.ReceiveHit`
  (params (MyComp :type "PrimitiveComponent Object Reference") (Other :type "Actor Object Reference") (OtherComp :type "PrimitiveComponent Object Reference") (bSelfMoved :type Boolean) (HitLocation :type "Vector Structure") (HitNormal :type "Vector Structure") (NormalImpulse :type "Vector Structure") (Hit :type "HitResult Structure (by ref)"))
  (`|SpawnActorFromClass` "/Game/TwinStickBP/Blueprints/Actors/BP_NovaHit.BP_NovaHit_C" (`KismetMathLibrary.MakeTransform` HitLocation (`KismetMathLibrary.Conv_VectorToRotator` HitNormal)) "Undefined" "OverrideRootScale" null (`self.DamagePower`))
  (bind _asbp_ship (cast `/Game/SpaceKatana/Blueprints/BP_Ship` Other)
    (:`then`
      (`/Game/SpaceKatana/Blueprints/BP_Ship.TakeDamge` _asbp_ship (`self.DamagePower`))
      (`self.K2_DestroyActor`))
    (:`CastFailed`
      (bind _asbp_module (cast `/Game/SpaceKatana/Blueprints/BP_Module` Other)
        (:`then`
          (`self.K2_DestroyActor` _asbp_module))
        (:`CastFailed`
          _))
      (`self.K2_DestroyActor`))))

(event `self.StaticMesh.OnComponentBeginOverlap`
  (params (OverlappedComponent :type "PrimitiveComponent Object Reference") (OtherActor :type "Actor Object Reference") (OtherComp :type "PrimitiveComponent Object Reference") (OtherBodyIndex :type Integer) (bFromSweep :type Boolean) (SweepResult :type "HitResult Structure (by ref)"))
  (`KismetSystemLibrary.PrintString` "Hello"))

(fn `UpdateMesh`
  (switch `/Game/SpaceKatana/DATA/Enums/ProjectileType` (`self.Type`)))

(fn `UserConstructionScript`
  (set `ProjectileMovementComponent.InitialSpeed` (`self.ProjectileInitSpeed`) (`self.ProjectileMovement`))
  (`self.UpdateMesh`))