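; BP_Module is a ship module in the space battle, with connector child actors and placeholder, flying-in and destroyed states.
; It follows GM_SpaceBattle events, easing to its target when modules spawn and coloring its lights green or red by root connection each turn.
; Destruction switches it to spinning physics freefall, pushed along +Y with clamped velocities while disconnected.
; Placeholders get a fly-in direction material and a spawn-order widget.
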(event `CustomEvent_3`
  (params (NewStep :type "ETurnStep Enum"))
  (switch `ETurnStep` NewStep
    (:`SpawningModules`
      (switch `EModuleState` (`self.CurrentState`)
        (:`STATE_FlyIn`
          (`KismetSystemLibrary.MoveComponentTo` (`self.K2_GetRootComponent`) (`self.TargetMoveTo`) (`self.K2_GetActorRotation`) true false 2.9))))))

(event `CustomEvent_1`
  (params (Time :type "Float (double-precision)") (TimeProgressed :type "Float (double-precision)"))
  (bind _staticmesh (`self.StaticMesh`))
  (bind _asgm_space_battle (cast `/Game/SpaceKatana/Blueprints/GM_SpaceBattle` (`GameplayStatics.GetGameMode`)))
  (switch `ETurnStep` (`GameModeBattle.CurrentStep` _asgm_space_battle)
    (:`Moving`
      _)
    (:`SpawningModules`
      _))
  (if (not (`self.bIsConnectedToRoot`))
    (switch `EModuleState` (`self.CurrentState`)
      (:`STATE_Destroyed`
        (if (`SceneComponent.IsSimulatingPhysics` (`self.StaticMesh`) "None")
          (`PrimitiveComponent.AddForce` _staticmesh (0.0 1500.0 0.0) "None" true)
          (`|ExecutionSequence`
            (:`then_0`
              (bind _returnvalue (`PrimitiveComponent.GetPhysicsLinearVelocity` _staticmesh "None"))
              (`PrimitiveComponent.SetPhysicsLinearVelocity` _staticmesh (`KismetMathLibrary.MakeVector` (`KismetMathLibrary.FClamp` (.x _returnvalue) -100.0 100.0) (`KismetMathLibrary.FClamp` (.y _returnvalue) -100.0 2000.0) (.z _returnvalue)) false "None"))
            (:`then_1`
              (bind _returnvalue_2 (`PrimitiveComponent.GetPhysicsAngularVelocity` _staticmesh "None"))
              (`PrimitiveComponent.SetPhysicsAngularVelocity` _staticmesh (`KismetMathLibrary.ClampVectorSize` _returnvalue_2 -100.0 100.0) false "None"))))))))

(event `self.ReceiveBeginPlay`
  (`|ExecutionSequence`
    (:`then_0`
      (for _array_element (`self.GetAllChildActors` false)
        (bind _asship_module_connector (cast `ShipModuleConnector` _array_element))
        (`KismetArrayLibrary.Array_Add` (`self.Connectors`) _asship_module_connector)))
    (:`then_1`
      (add `self.OnShipModuleDestroyed` (delegate `CustomEvent_0`))
      (bind _asgm_space_battle (cast `/Game/SpaceKatana/Blueprints/GM_SpaceBattle` (`GameplayStatics.GetGameMode`)))
      (add `/Game/SpaceKatana/Blueprints/GM_SpaceBattle.OnNewTurn` _asgm_space_battle (delegate `CustomEvent_2`))
      (bind _asgm_space_battle_2 (cast `/Game/SpaceKatana/Blueprints/GM_SpaceBattle` (`GameplayStatics.GetGameMode`)))
      (add `/Game/SpaceKatana/Blueprints/GM_SpaceBattle.TimeUpdated` _asgm_space_battle_2 (delegate `CustomEvent_1`))
      (add `/Game/SpaceKatana/Blueprints/GM_SpaceBattle.OnStepChange` _asgm_space_battle_2 (delegate `CustomEvent_3`)))))

(event `CustomEvent_2`
  (bind _children (`SceneComponent.GetChildrenComponents` (`self.K2_GetRootComponent`) false))
  (if (`self.bIsConnectedToRoot`)
    (for _array_element _children
      (bind _aslight_component (cast `LightComponent` _array_element))
      (`LightComponent.SetLightColor` _aslight_component (struct :`G` 1.0 :`B` 0.041734 :`A` 1.0) true))
    (else
      (for _array_element_2 _children
        (bind _aslight_component_2 (cast `LightComponent` _array_element_2))
        (`LightComponent.SetLightColor` _aslight_component_2 (struct :`R` 1.0 :`B` 0.012242 :`A` 1.0) true)))))

(event `CustomEvent_0` :!signature `self.OnShipModuleDestroyed`
  (params (Module :type "ShipModule Object Reference"))
  (`self.SetFreefallMode`))

(event `self.ReceiveTick`
  (params (DeltaSeconds :type "Float (single-precision)"))
  ;[1 1 1] Tick
)

(event `self.InitModule`
  ;[1 1 1] Init Module
  (`parent.InitModule`)
  (switch `EModuleState` (`self.CurrentState`)
    (:`STATE_Placeholder`
      (`self.SetPlaceholderMode`))))

(fn `SetFlyInMode`
  (bind _staticmesh (`self.StaticMesh`))
  (`PrimitiveComponent.SetSimulatePhysics` _staticmesh true)
  (`PrimitiveComponent.SetConstraintMode` _staticmesh "XYPlane")
  (`PrimitiveComponent.SetPhysicsLinearVelocity` (`self.StaticMesh`) (* (`self.FlyInDirection`) 300.0) false "None"))

(fn `SetFreefallMode`
  (bind _staticmesh (`self.StaticMesh`))
  (`PrimitiveComponent.SetSimulatePhysics` _staticmesh true)
  (`PrimitiveComponent.SetCollisionEnabled` _staticmesh "PhysicsOnly")
  (`PrimitiveComponent.AddTorque` _staticmesh (`KismetMathLibrary.MakeVector` 0.0 0.0 (`KismetMathLibrary.RandomFloatInRange` -50.0 50.0)) "None" true)
  (set `self.CurrentState` "STATE_Destroyed"))

(fn `SetPlaceholderMode`
  (set `self.CurrentState` "STATE_Placeholder")
  (bind _returnvalue (`PrimitiveComponent.CreateDynamicMaterialInstance` (`self.StaticMesh`) 0 "/Game/SpaceKatana/Materials/M_FlyinDirection.M_FlyinDirection"))
  (set `self.PlaceholderDynamicMaterialInstance` _returnvalue)
  (bind _aswidget_order_visualizer (cast `/Game/SpaceKatana/Hud/Widget/Widget_OrderVisualizer` (`WidgetComponent.GetUserWidgetObject` (`self.ModuleWidget`))))
  (`SceneComponent.SetHiddenInGame` (`self.ModuleWidget`) false false)
  (set `/Game/SpaceKatana/Hud/Widget/Widget_OrderVisualizer.Order` (`self.SpawnOrder`) _aswidget_order_visualizer))

(fn `UserConstructionScript`)