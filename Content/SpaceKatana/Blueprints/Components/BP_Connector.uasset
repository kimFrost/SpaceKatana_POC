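; BP_Connector is a child actor of BP_Module that snaps an incoming module onto an attached one.
; When its sphere overlaps another connector while its parent is "Flying in" and the other's parent is Attached, it sets its parent to Attached.
; It then teleports that parent 100 units from the attached module toward the touched connector.
; A legacy JoinOld function does similar positioning for BP_Module_OLD.
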(event `self.ReceiveTick`
  (params (DeltaSeconds :type "Float (single-precision)")))

(event `self.Sphere.OnComponentBeginOverlap`
  (params (OverlappedComponent :type "PrimitiveComponent Object Reference") (OtherActor :type "Actor Object Reference") (OtherComp :type "PrimitiveComponent Object Reference") (OtherBodyIndex :type Integer) (bFromSweep :type Boolean) (SweepResult :type "HitResult Structure (by ref)"))
  (bind _asbp_module (cast `/Game/SpaceKatana/Blueprints/BP_Module` (`self.GetParentActor`)))
  (switch `EModuleState` (`ShipModule.CurrentState` _asbp_module)
    (:`STATE_FlyIn`
      (bind _asbp_connector (cast `/Game/SpaceKatana/Blueprints/Components/BP_Connector` OtherActor))
      (bind _asbp_module_2 (cast `/Game/SpaceKatana/Blueprints/BP_Module` (`self.GetParentActor` _asbp_connector)))
      (switch `EModuleState` (`ShipModule.CurrentState` _asbp_module_2)
        (:`STATE_Attached`
          (set `ShipModule.CurrentState` "STATE_Attached" _asbp_module)
          (bind _returnvalue (`self.K2_GetActorLocation` _asbp_module_2))
          (`self.K2_SetActorLocation` _asbp_module (+ _returnvalue (* (`KismetMathLibrary.GetDirectionVector` _returnvalue (`self.K2_GetActorLocation` _asbp_connector)) 100.0)) false true))))))

(fn `Join_Old`
  (params (Connector :type "/Game/SpaceKatana/Blueprints/Components/BP_Connector Object Reference") (UpdateParentLocation :type Boolean) (UpdateOther :type Boolean))
  (`/Engine/EditorBlueprintResources/StandardMacros.IsValid` Connector
    (:`Is Valid`
      (if (!= Connector (`self.OtherConnector`))
        (`|ExecutionSequence`
          (:`then_0`
            (if UpdateOther
              (`self.Join_Old` Connector self false false)))
          (:`then_1`
            (if UpdateParentLocation
              (bind _asbp_module_old (cast `/Game/SpaceKatana/Blueprints/BP_Module_OLD` (`self.GetParentActor` Connector)))
              (bind _asbp_module_old_2 (cast `/Game/SpaceKatana/Blueprints/BP_Module_OLD` (`self.GetParentActor`)))
              (`self.K2_SetActorLocation` _asbp_module_old (+ (`self.K2_GetActorLocation` _asbp_module_old_2) (* (`self.GetActorForwardVector`) 100.0)) false false))))))))

(fn `UserConstructionScript`)