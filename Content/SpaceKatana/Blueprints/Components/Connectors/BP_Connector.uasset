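; BP_Connector is a connection point parented to a module actor, used to join modules together.
; JoinOld calls itself reciprocally on the other connector and can snap that connector's BP_Module_OLD parent a fixed distance along this connector's forward vector, but its OtherConnector assignment is disconnected.
; The overlap event is empty, leaving the newer BP_Module logic for snapping flying modules onto attached ones unreachable, along with the debug drawing.
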(event `self.Sphere.OnComponentBeginOverlap`
  (params (OverlappedComponent :type "PrimitiveComponent Object Reference") (OtherActor :type "Actor Object Reference") (OtherComp :type "PrimitiveComponent Object Reference") (OtherBodyIndex :type Integer) (bFromSweep :type Boolean) (SweepResult :type "HitResult Structure (by ref)")))

(fn `Join_Old`
  (params (Connector :type "/Game/SpaceKatana/Blueprints/Components/Connectors/BP_Connector Object Reference") (UpdateParentLocation :type Boolean) (UpdateOther :type Boolean))
  (`/Engine/EditorBlueprintResources/StandardMacros.IsValid` Connector
    (:`Is Valid`
      (if (!= Connector (`self.OtherConnector`))
        (`|ExecutionSequence`
          (:`then_0`
            (if UpdateOther
              (`self.Join_Old` Connector self false false)))
          (:`then_1`
            (if UpdateParentLocation
              (bind _asbp_module_old (cast `/Game/SpaceKatana/Blueprints/BP_Module_OLD` (`self.GetParentActor` Connector)))
              (bind _asbp_module_old_2 (cast `/Game/SpaceKatana/Blueprints/BP_Module_OLD` (`self.GetParentActor`)))
              (`self.K2_SetActorLocation` _asbp_module_old (+ (`self.K2_GetActorLocation` _asbp_module_old_2) (* (`self.GetActorForwardVector`) 100.0)) false false))))))))

(fn `UserConstructionScript`)