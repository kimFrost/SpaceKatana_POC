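; Game mode for a turn-based space battle that builds the tile grid and runs the turn clock.
; Tick advances a countdown that steps through planning, moving, shooting, module spawning and maneuvering, broadcasting changes; both players readying up zeroes it.
; New turns reset readiness, age orders and update modules.
; SetPlayRate offsets global time dilation for itself, and Tick also debug-draws the tile under the mouse.
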(event `self.ReceiveTick`
  (params (DeltaSeconds :type "Float (single-precision)"))
  (bind _playrate (`self.PlayRate`))
  (bind (_worldlocation _worlddirection) (`PlayerController.DeprojectMousePositionToWorld` (`GameplayStatics.GetPlayerController` 0)))
  (bind (_t _intersection) (`KismetMathLibrary.LinePlaneIntersection_OriginNormal` _worldlocation (+ _worldlocation (* _worlddirection 10000.0)) (0.0 0.0 0.0) (0.0 1.0 0.0)))
  (`|ExecutionSequence`
    (:`then_0`
      (if (> _playrate 0.0001)
        (`self.ProgressTime` (* DeltaSeconds _playrate))))
    (:`then_1`
      (`KismetSystemLibrary.DrawDebugSphere` _intersection 10.0 12 (struct :`R` 0.302893 :`G` 0.02717 :`B` 1.0 :`A` 1.0) 0.0 10.0)
      (bind _returnvalue (`self.GetGridTile` _intersection true))
      (`/Engine/EditorBlueprintResources/StandardMacros.IsValid` _returnvalue
        (:`Is Valid`
          (set `GridTile.bDebugMe` true _returnvalue))))
    (:`then_2`
      (for _array_element (`self.GridTiles`)
        (bind _bdebugme (`GridTile.bDebugMe` _array_element))
        (if _bdebugme
          (`KismetSystemLibrary.DrawDebugBox` (+ (`GridTile.WorldLocation` _array_element) (/ (`self.GridTileSize`) 2.0)) (45.0 0.0 45.0) (`KismetMathLibrary.SelectColor` (struct :`R` 1.0 :`G` 0.666656 :`A` 1.0) (struct :`R` 0.07 :`B` 0.012466 :`A` 1.0) _bdebugme) (struct) 0.0 (`KismetMathLibrary.SelectFloat` 10.0 3.0 _bdebugme))
          (set `GridTile.bDebugMe` false _array_element))))))

(event `self.ReceiveBeginPlay`
  (`self.ConstructGrid`)
  (`KismetSystemLibrary.Delay` 0.5)
  (`self.NewTurn`))

(fn `EndTurn`
  (params (ShipIndex :type Integer))
  (switch `int` ShipIndex
    (:`0`
      (set `self.PlayerOneReady` true))
    (:`1`
      (set `self.PlayerTwoReady` true)))
  (if (and (`self.PlayerOneReady`) (`self.PlayerTwoReady`))
    (set `self.TurnTimeLeft` 0.0)))

(fn `NewTurn`
  (set `self.PlayerOneReady` false)
  (set `self.PlayerTwoReady` false)
  (set `self.HighestSequence` 0)
  (for _array_element (`self.Orders`)
    (`/Engine/EditorBlueprintResources/StandardMacros.IsValid` _array_element
      (:`Is Valid`
        (`/Engine/EditorBlueprintResources/StandardMacros.DecrementInt` (`Order.TurnsLeft` _array_element)))))
  (set `self.CurrentStep` "Planning")
  (set `self.TurnTimeLeft` (`self.PlaningLength`))
  (`self.UpdateAllModules`)
  (`self.OnNewTurn`))

(fn `ProgressTime`
  (params (Amount :type "Float (double-precision)"))
  (bind _output_get (set `self.Time` (+ Amount (`self.Time`))))
  (`|ExecutionSequence`
    (:`then_0`
      (bind _output_get_2 (set `self.TurnTimeLeft` (- (`self.TurnTimeLeft`) Amount)))
      (if (<= _output_get_2 0.0)
        (`|ExecutionSequence`
          (:`then_0`
            (bind _returnvalue (`self.ProgressTurnStep`))
            (switch `ETurnStep` _returnvalue
              (:`Planning`
                (`self.NewTurn`))
              (:`Moving`
                (set `self.TurnTimeLeft` 1.0)
                (`self.SetPlayRate` 1.0 1.0))
              (:`Shooting`
                (set `self.TurnTimeLeft` 1.0))
              (:`SpawningModules`
                (set `self.TurnTimeLeft` 1.0)
                (`self.UpdateOrders` "SpawnModule"))
              (:`Maneuvering`
                (set `self.TurnTimeLeft` 2.0))))
          (:`then_1`
            (`self.OnStepChange` (`self.CurrentStep`))))))
    (:`then_1`
      (`self.TimeUpdated` _output_get Amount))))

(fn `SetPlayRate`
  (params (TimeRate :type "Float (double-precision)") (DilationRate :type "Float (double-precision)"))
  (set `self.PlayRate` TimeRate)
  (`GameplayStatics.SetGlobalTimeDilation` DilationRate)
  ;[1 1 1] Override the effect of dilation in this gamemode
  (set `self.CustomTimeDilation` (/ 1.0 (`GameplayStatics.GetGlobalTimeDilation`))))

(fn `UserConstructionScript`)