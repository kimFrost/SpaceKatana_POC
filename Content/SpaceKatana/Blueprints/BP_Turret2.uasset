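; Ship-mounted turret for BP_Ship that aims at a target location, with yaw clamped to an arc around its mount.
; Priming drains the ship's power, and resetting the target refunds it if still primed.
; Fire waits a wind-up, then spawns a timed burst of shell or laser projectiles with accuracy-based random spread.
; Debug draw calls show the firing arc and aim direction unless the ship hides its UI.
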(event `self.ReceiveBeginPlay`
  (bind _asbp_ship (cast `/Game/SpaceKatana/Blueprints/BP_Ship` (`self.GetParentActor`)))
  (set `self.Ship` _asbp_ship)
  (set `self.AttachedToShip` true))

(event `self.ReceiveTick`
  (params (DeltaSeconds :type "Float (single-precision)"))
  (bind _returnvalue (`self.K2_GetActorLocation`))
  (bind _ship (`self.Ship`))
  (if (`self.AttachedToShip`)
    (`/Engine/EditorBlueprintResources/StandardMacros.IsValid` _ship
      (:`Is Valid`
        (if (not (`/Game/SpaceKatana/Blueprints/BP_Ship.HideUI` _ship))
          (`|ExecutionSequence`
            (:`then_0`
              (if (`self.Targeting`)
                (`KismetSystemLibrary.DrawDebugConeInDegrees` (`self.K2_GetActorLocation`) (`KismetMathLibrary.GreaterGreater_VectorRotator` (`SceneComponent.GetForwardVector` (`self.DefaultSceneRoot`)) (struct :`Yaw` 180.0)) 200.0 (/ (+ (`KismetMathLibrary.Abs` (`self.MinAngle`)) (`self.MaxAngle`)) 2.0) 0.0 2)))
            (:`then_1`
              (bind _asbp_ship (cast `/Game/SpaceKatana/Blueprints/BP_Ship` (`self.GetParentActor`)))
              (if (and (`|EnumEquality` (`/Game/SpaceKatana/Blueprints/BP_Ship.Mode` _asbp_ship) "NewEnumerator1") (or (`self.Primed`) (`self.Targeting`)))
                (`KismetSystemLibrary.DrawDebugArrow` _returnvalue (+ _returnvalue (* (`self.ClampedDirection`) 200.0)) 30.0 (struct :`R` 1.0 :`B` 0.009549 :`A` 1.0) 0.0 2.0)))))))))

(event `Fire`
  (bind _shotsleft (`self.ShotsLeft`))
  (`/Engine/EditorBlueprintResources/StandardMacros.IsValid` (`self.Ship`)
    (:`Is Valid`
      (set `self.ShotsLeft` (`self.ShotsToFire`))
      (`KismetSystemLibrary.Delay` (`self.WindUpTime`))
      (`self.FireProjectile` :!label _label)
      (`/Engine/EditorBlueprintResources/StandardMacros.DecrementInt` _shotsleft
        (:`  `
          (if (> _shotsleft 0)
            (`KismetSystemLibrary.Delay` 0.2)
            (goto _label)
            (else
              (set `self.LockAndLoaded` false))))))))

(fn `ActivateTargeting`
  (set `self.Targeting` true))

(fn `FireProjectile`
  (bind _ship (`self.Ship`))
  (bind _ship_2 (`self.Ship`))
  (bind _returnvalue (/ (- 100.0 (`self.AccuracyProcent`)) 2.0))
  (bind _returnvalue_2 (`KismetMathLibrary.MakeTransform` (`SceneComponent.K2_GetComponentLocation` (`self.Cannon`)) (`KismetMathLibrary.ComposeRotators` (`KismetMathLibrary.ComposeRotators` (`SceneComponent.K2_GetComponentRotation` (`self.StaticMesh_0`)) (struct :`Yaw` 180.0)) (`KismetMathLibrary.MakeRotator` 0.0 0.0 (`KismetMathLibrary.RandomFloatInRange` (* _returnvalue -1.0) _returnvalue))) (1.0 1.0 1.0)))
  (switch `/Game/SpaceKatana/DATA/Enums/ProjectileType` (`self.ProjectileType`)
    (:`NewEnumerator0`
      (`|SpawnActorFromClass` "/Game/SpaceKatana/Blueprints/BP_ProjectileShell.BP_ProjectileShell_C" _returnvalue_2 "Undefined" "OverrideRootScale" _ship (`self.ProjectileSpeed`) (`self.ProjectileDamagePower`) "NewEnumerator0" _ship)
      (set `self.Primed` false))
    (:`NewEnumerator2`
      (`|SpawnActorFromClass` "/Game/SpaceKatana/Blueprints/BP_ProjectileLaser.BP_ProjectileLaser_C" _returnvalue_2 "Undefined" "OverrideRootScale" _ship_2 (`self.ProjectileSpeed`) (`self.ProjectileDamagePower`) "NewEnumerator2" _ship_2)
      (set `self.Primed` false))))

(fn `PrimeTurret`
  (bind _ship (`self.Ship`))
  (if (not (`self.Primed`))
    (`/Engine/EditorBlueprintResources/StandardMacros.IsValid` _ship
      (:`Is Valid`
        (bind _drained (`/Game/SpaceKatana/Blueprints/BP_Ship.DrainPower` _ship (`self.FirePowerCost`)))
        (set `self.Primed` _drained)))))

(fn `ResetTargetLocation`
  (bind _ship (`self.Ship`))
  (set `self.TargetLocation` (0.0 0.0 0.0))
  (set `self.RelativeTargetLocation` (1.0 0.0 0.0))
  (set `self.Targeting` false)
  (if (`self.Primed`)
    ;[1 1 1] Refund power
    (set `self.Primed` false)
    (`/Engine/EditorBlueprintResources/StandardMacros.IsValid` _ship
      (:`Is Valid`
        (`/Game/SpaceKatana/Blueprints/BP_Ship.AddPower` _ship (`self.FirePowerCost`)))))
  (`self.UpdateTurret`))

(fn `SetTargetLocation`
  (params (Location :type "Vector Structure"))
  (bind _output_get (set `self.TargetLocation` (`KismetMathLibrary.MakeVector` (.x Location) (.y Location))))
  (set `self.RelativeTargetLocation` (- _output_get (`self.K2_GetActorLocation`)))
  (`self.UpdateTurret`))

(fn `UpdateTurret`
  (bind _yaw (.yaw (`SceneComponent.K2_GetComponentRotation` (`self.DefaultSceneRoot`))))
  (bind _output_get (set `self.ClampedTargetAngle` (`KismetMathLibrary.FClamp` (.yaw (`KismetMathLibrary.FindLookAtRotation` (`self.RelativeTargetLocation`) (`KismetMathLibrary.MakeVector` 0.0))) (+ _yaw (`self.MinAngle`)) (+ _yaw (`self.MaxAngle`)))))
  (`SceneComponent.K2_SetWorldRotation` (`self.StaticMesh_0`) (`KismetMathLibrary.MakeRotator` 0.0 0.0 _output_get) false false)
  (set `self.ClampedDirection` (`KismetMathLibrary.GetForwardVector` (`KismetMathLibrary.ComposeRotators` (`KismetMathLibrary.MakeRotator` 0.0 0.0 (`self.ClampedTargetAngle`)) (struct :`Yaw` 180.0))))
  (`KismetSystemLibrary.DrawDebugPoint` (`self.TargetLocation`) 5.0 (struct) 0.0))

(fn `UserConstructionScript`)