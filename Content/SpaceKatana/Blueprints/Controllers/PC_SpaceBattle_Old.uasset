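; Player controller for space battles that gives mouse orders to ships and their turrets.
; Left-click selects a ship or turret and switches the ship's mode; clicking elsewhere commits a destination, or a target that primes the turret.
; While selected, Tick feeds the cursor trace hit to the actor as a live destination or aim point.
; Right-click resets the selected or hovered actor's order; leftover possession and movement-field nodes never run.
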(event `self.ReceiveTick`
  (params (DeltaSeconds :type "Float (single-precision)"))
  (bind _selectedactor (`self.SelectedActor`))
  (bind (_bblockinghit _binitialoverlap _time _location) (`GameplayStatics.BreakHitResult` (`self.GetHitResultUnderCursorByChannel` "TraceTypeQuery1")))
  (`/Engine/EditorBlueprintResources/StandardMacros.IsValid` (`self.SelectedActor`)
    (:`Is Valid`
      (bind _asbp_turret (cast `/Game/SpaceKatana/Blueprints/Modules/BP_Turret` _selectedactor)
        (:`then`
          (`/Game/SpaceKatana/Blueprints/Modules/BP_Turret.SetTargetLocation` _asbp_turret _location))
        (:`CastFailed`
          (bind _asbp_ship (cast `/Game/SpaceKatana/Blueprints/BP_Ship` _selectedactor))
          (`/Game/SpaceKatana/Blueprints/BP_Ship.SetDestination` _asbp_ship _location))))))

(event `Key|LeftMouseButton`
  (params (Key :type "Key Structure" :default "AnyKey"))
  (bind (_hitresult _returnvalue) (`self.GetHitResultUnderCursorByChannel` "TraceTypeQuery1"))
  (bind _selectedactor (`self.SelectedActor`))
  (bind (_bblockinghit _binitialoverlap _time _location _impactpoint _normal _impactnormal _physmat _hitactor) (`GameplayStatics.BreakHitResult` _hitresult))
  (:`Pressed`
    (if _returnvalue
      (bind _asbp_ship (cast `/Game/SpaceKatana/Blueprints/BP_Ship` _hitactor)
        (:`then`
          (set `self.SelectedActor` _asbp_ship)
          (set `/Game/SpaceKatana/Blueprints/BP_Ship.Mode` "NewEnumerator0" _asbp_ship))
        (:`CastFailed`
          (bind _asbp_turret (cast `/Game/SpaceKatana/Blueprints/Modules/BP_Turret` _hitactor)
            (:`then`
              (bind _output_get (set `self.SelectedActor` _asbp_turret))
              (set `/Game/SpaceKatana/Blueprints/Modules/BP_Turret.Targeting` true _asbp_turret)
              (bind _asbp_ship_2 (cast `/Game/SpaceKatana/Blueprints/BP_Ship` (`self.GetParentActor` _output_get)))
              (set `/Game/SpaceKatana/Blueprints/BP_Ship.Mode` "NewEnumerator1" _asbp_ship_2))
            (:`CastFailed`
              (bind _asbp_ship_3 (cast `/Game/SpaceKatana/Blueprints/BP_Ship` _selectedactor)
                (:`then`
                  (`/Game/SpaceKatana/Blueprints/BP_Ship.SetDestination` _asbp_ship_3 _location)
                  (set `/Game/SpaceKatana/Blueprints/BP_Ship.Mode` "NewEnumerator0" _asbp_ship_3)
                  (set `self.SelectedActor` null))
                (:`CastFailed`
                  (bind _asbp_turret_2 (cast `/Game/SpaceKatana/Blueprints/Modules/BP_Turret` _selectedactor))
                  (`/Game/SpaceKatana/Blueprints/Modules/BP_Turret.SetTargetLocation` _asbp_turret_2 _location)
                  (set `/Game/SpaceKatana/Blueprints/Modules/BP_Turret.Targeting` false _asbp_turret_2)
                  (`/Game/SpaceKatana/Blueprints/Modules/BP_Turret.PrimeTurret` _asbp_turret_2)
                  (set `self.SelectedActor` null))))))))))

(event `Key|RightMouseButton`
  (params (Key :type "Key Structure" :default "AnyKey"))
  (bind (_hitresult _returnvalue) (`self.GetHitResultUnderCursorByChannel` "TraceTypeQuery1"))
  (bind _selectedactor (`self.SelectedActor`))
  (bind (_bblockinghit _binitialoverlap _time _location _impactpoint _normal _impactnormal _physmat _hitactor) (`GameplayStatics.BreakHitResult` _hitresult))
  (:`Pressed`
    (`/Engine/EditorBlueprintResources/StandardMacros.IsValid` (`self.SelectedActor`)
      (:`Is Valid`
        (bind _asbp_turret (cast `/Game/SpaceKatana/Blueprints/Modules/BP_Turret` _selectedactor)
          (:`then`
            (`/Game/SpaceKatana/Blueprints/Modules/BP_Turret.ResetTargetLocation` _asbp_turret)
            (set `self.SelectedActor` null))
          (:`CastFailed`
            (bind _asbp_ship (cast `/Game/SpaceKatana/Blueprints/BP_Ship` _selectedactor))
            (`/Game/SpaceKatana/Blueprints/BP_Ship.ResetTravel` _asbp_ship)
            (set `self.SelectedActor` null))))
      (:`Is Not Valid`
        (if _returnvalue
          (bind _asbp_ship_2 (cast `/Game/SpaceKatana/Blueprints/BP_Ship` _hitactor)
            (:`then`
              (`/Game/SpaceKatana/Blueprints/BP_Ship.ResetTravel` _asbp_ship_2))
            (:`CastFailed`
              (bind _asbp_turret_2 (cast `/Game/SpaceKatana/Blueprints/Modules/BP_Turret` _hitactor))
              (`/Game/SpaceKatana/Blueprints/Modules/BP_Turret.ResetTargetLocation` _asbp_turret_2))))))))

(fn `UserConstructionScript`)