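; Player controller for the space battle mode that lets the player place and cancel module spawn orders on a tile grid during the Planning step.
; Tick projects the mouse onto the Y-normal plane and fires a tile-focus event that moves the pending order's coordinates and fly-in direction.
; R rotates the direction, left click drops the placeholder, right click cancels orders.
; Each new turn assigns ship index 1; older ship/turret click controls remain disconnected.
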(event `self.ReceiveTick`
  (params (DeltaSeconds :type "Float (single-precision)"))
  (bind (_worldlocation _worlddirection) (`self.DeprojectMousePositionToWorld`))
  (bind (_worldlocation_2 _worlddirection_2) (`self.DeprojectMousePositionToWorld`))
  (bind (_t _intersection) (`KismetMathLibrary.LinePlaneIntersection_OriginNormal` _worldlocation_2 (+ _worldlocation_2 (* _worlddirection_2 10000.0)) (0.0 0.0 0.0) (0.0 1.0 0.0)))
  (`|ExecutionSequence`
    (:`then_0`
      (bind _asgm_space_battle (cast `/Game/SpaceKatana/Blueprints/GameModes/GM_SpaceBattle` (`GameplayStatics.GetGameMode`)))
      (bind _returnvalue (`GameModeBattle.WorldLocationToCoords` _asgm_space_battle (- (`.Intersection` (`KismetMathLibrary.LinePlaneIntersection_OriginNormal` _worldlocation (+ _worldlocation (* _worlddirection 10000.0)) (0.0 0.0 0.0) (0.0 1.0 0.0))) (* (`self.SpawnInDirection`) 25000.0)) true))
      (if (not (== _returnvalue (`self.LastFocusTileCoords`)))
        (bind _output_get (set `self.LastFocusTileCoords` _returnvalue))
        (`self.OnTileFocus` (`KismetMathLibrary.FTrunc` (.x _output_get)) (`KismetMathLibrary.FTrunc` (.z _output_get)))))
    (:`then_1`
      (`KismetSystemLibrary.DrawDebugArrow` _intersection (+ _intersection (* (`self.SpawnInDirection`) 100.0)) 100.0 (struct :`G` 0.032635 :`B` 1.0 :`A` 1.0) 0.0 5.0))
    (:`then_2`
      (`KismetSystemLibrary.PrintString` (`KismetStringLibrary.BuildString_Int` "Controlling: " (`KismetSystemLibrary.GetDisplayName` (`self.Ship`))) true false (struct :`G` 0.66 :`B` 1.0 :`A` 1.0) 0.0))))

(event `Key|LeftMouseButton`
  (params (Key :type "Key Structure" :default "AnyKey"))
  (:`Pressed`
    (switch `EToolType` (`self.CurrentTool`)
      (:`SpawnModule`
        ;[1 1 1] Let go off spawn tool. Let placeholder stay in place
        (`/Engine/EditorBlueprintResources/StandardMacros.IsValid` (`self.SpawnOrder`)
          (:`Is Valid`
            (set `self.SpawnOrder` null)
            (`self.SetTool` "Select")))))))

(event `Key|R`
  (params (Key :type "Key Structure" :default "AnyKey"))
  (:`Pressed`
    (`self.RotateDirection`)))

(event `Key|RightMouseButton`
  (params (Key :type "Key Structure" :default "AnyKey"))
  (:`Pressed`
    (bind _asgm_space_battle (cast `/Game/SpaceKatana/Blueprints/GameModes/GM_SpaceBattle` (`GameplayStatics.GetGameMode`)))
    (switch `ETurnStep` (`GameModeBattle.CurrentStep` _asgm_space_battle)
      (:`Planning`
        (switch `EToolType` (`self.CurrentTool`)
          (:`Select`
            (bind _asbp_module (cast `/Game/SpaceKatana/Blueprints/BP_Module` (`.HitActor` (`GameplayStatics.BreakHitResult` (`self.GetHitResultUnderCursorForObjects` (`|MakeArray` "ObjectTypeQuery9" :!type "EObjectTypeQuery Enum"))))))
            (switch `EModuleState` (`ShipModule.CurrentState` _asbp_module)
              (:`STATE_Placeholder`
                (bind _spawnorder (`ShipModule.SpawnOrder` _asbp_module))
                (`/Engine/EditorBlueprintResources/StandardMacros.IsValid` _spawnorder
                  (:`Is Valid`
                    (`Order.CancelOrder` _spawnorder))))))
          (:`SpawnModule`
            ;[1 1 1] Cancel Current Tool
            (`self.CancelToolOrder`)
            (`self.SetTool` "Select")))))))

(event `self.ReceiveBeginPlay`
  (`|ExecutionSequence`
    (:`then_0`
      (bind _asgm_space_battle (cast `/Game/SpaceKatana/Blueprints/GameModes/GM_SpaceBattle` (`GameplayStatics.GetGameMode`)))
      (add `GameModeBattle.OnNewTurn` _asgm_space_battle (delegate `CustomEvent_1`)))
    (:`then_1`
      (add `self.OnTileFocus` (delegate `CustomEvent_0`)))))

(event `CustomEvent_1`
  (bind _ship (`self.GetShipRef` 1))
  (`self.ControlShip` _ship))

(event `CustomEvent_0` :!signature `self.OnTileFocus`
  (params (X :type Integer) (Z :type Integer))
  (bind (_worldlocation _worlddirection) (`self.DeprojectMousePositionToWorld`))
  (bind _spawnorder (`self.SpawnOrder`))
  (`/Engine/EditorBlueprintResources/StandardMacros.IsValid` (`self.SpawnOrder`)
    (:`Is Valid`
      (bind _asgm_space_battle (cast `/Game/SpaceKatana/Blueprints/GameModes/GM_SpaceBattle` (`GameplayStatics.GetGameMode`)))
      (switch `ETurnStep` (`GameModeBattle.CurrentStep` _asgm_space_battle)
        (:`Planning`
          (bind _returnvalue (`GameModeBattle.WorldLocationToCoords` _asgm_space_battle (- (`.Intersection` (`KismetMathLibrary.LinePlaneIntersection_OriginNormal` _worldlocation (+ _worldlocation (* _worlddirection 10000.0)) (0.0 0.0 0.0) (0.0 1.0 0.0))) (* (`self.SpawnInDirection`) 25000.0)) true))
          (set `OrderSpawnModule.FlyInDirection` (`self.SpawnInDirection`) _spawnorder)
          (set `Order.X` (`KismetMathLibrary.FTrunc` (.x _returnvalue)) _spawnorder)
          (set `Order.Z` (`KismetMathLibrary.FTrunc` (.z _returnvalue)) _spawnorder)
          (`OrderSpawnModule.TraceProjection` _spawnorder))))))

(fn `CancelToolOrder`
  (bind _spawnorder (`self.SpawnOrder`))
  (`/Engine/EditorBlueprintResources/StandardMacros.IsValid` _spawnorder
    (:`Is Valid`
      (`Order.CancelOrder` _spawnorder)
      (set `self.SpawnOrder` null))))

(fn `ControlShip`
  (params (Ship :type "/Game/SpaceKatana/Blueprints/BP_Ship Object Reference"))
  (set `self.Ship` Ship)
  (`/Engine/EditorBlueprintResources/StandardMacros.IsValid` Ship))

(fn `GetShipRef`
  (params (ShipIndex :type Integer))
  (returns (Ship :type "/Game/SpaceKatana/Blueprints/BP_Ship Object Reference"))
  (bind _outactors (`GameplayStatics.GetAllActorsOfClass` "/Game/SpaceKatana/Blueprints/BP_Ship.BP_Ship_C"))
  (for _array_element _outactors
    (if (== (`/Game/SpaceKatana/Blueprints/BP_Ship.Index` _array_element) ShipIndex)
      (return _array_element)))
  (return null))

(fn `RotateDirection`
  (set `self.SpawnInDirection` (`KismetMathLibrary.RotateAngleAxis` (`self.SpawnInDirection`) 90.0 (0.0 1.0 0.0))))

(fn `SetTool`
  (params (Type :type "EToolType Enum"))
  (`self.CancelToolOrder`)
  (bind _output_get (set `self.CurrentTool` Type))
  (switch `EToolType` _output_get
    (:`Select`
      (set `self.SpawnOrder` null))
    (:`SpawnModule`
      (bind _asgm_space_battle (cast `/Game/SpaceKatana/Blueprints/GameModes/GM_SpaceBattle` (`GameplayStatics.GetGameMode`)))
      (switch `ETurnStep` (`GameModeBattle.CurrentStep` _asgm_space_battle)
        (:`Planning`
          (bind _returnvalue (`GameModeBattle.AddOrder_SpawnModule` _asgm_space_battle (`self.SpawnModuleClass`) 0 0 (`self.SpawnInDirection`) null))
          (set `self.SpawnOrder` _returnvalue))))))

(fn `UserConstructionScript`)