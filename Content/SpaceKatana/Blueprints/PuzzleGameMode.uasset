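; Game mode for a two-player simultaneous-turn ship game, alternating timed Planning and Executing phases.
; Planning ends when both players are ready or time runs out, and Executing returns to a new turn on timeout.
; SetPlayRate sets global time dilation to zero for planning and normal for execution, inversely scaling its own dilation so Tick keeps counting.
; Dispatchers announce turn changes and time updates, while Tick prints debug values.
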(event `self.ReceiveTick`
  (params (DeltaSeconds :type "Float (single-precision)"))
  (bind _playrate (`self.PlayRate`))
  (if (> _playrate 0.0)
    (`self.ProgressTime` (* DeltaSeconds _playrate))
    (`KismetSystemLibrary.PrintString` (`KismetStringLibrary.Conv_DoubleToString` DeltaSeconds) true true (struct :`G` 0.199378 :`B` 1.0 :`A` 1.0) 0.0)
    (`KismetSystemLibrary.PrintString` (`KismetStringLibrary.Conv_DoubleToString` (`GameplayStatics.GetGlobalTimeDilation`)) true true (struct :`G` 0.66 :`B` 1.0 :`A` 1.0) 0.0)))

(event `self.ReceiveBeginPlay`
  (`self.NewTurn`))

(fn `EndTurn`
  (params (ShipIndex :type Integer))
  (switch `int` ShipIndex
    (:`0`
      (set `self.PlayerOneReady` true))
    (:`1`
      (set `self.PlayerTwoReady` true)))
  (if (and (`self.PlayerOneReady`) (`self.PlayerTwoReady`))
    (set `self.TurnStep` "NewEnumerator1")
    (set `self.TurnTimeLeft` (`self.PlayingLength`))
    (`self.SetPlayRate` 1.0 1.0)
    (`self.OnEndTurn`)))

(fn `NewTurn`
  (set `self.PlayerOneReady` false)
  (set `self.PlayerTwoReady` false)
  (set `self.TurnStep` "NewEnumerator0")
  (set `self.TurnTimeLeft` (`self.PlaningLength`))
  (`self.SetPlayRate` 1.0 0.0)
  (`self.OnNewTurn`))

(fn `ProgressTime`
  (params (Amount :type "Float (double-precision)"))
  (bind _output_get (set `self.Time` (+ Amount (`self.Time`))))
  (`|ExecutionSequence`
    (:`then_0`
      (bind _output_get_2 (set `self.TurnTimeLeft` (- (`self.TurnTimeLeft`) Amount)))
      (if (<= _output_get_2 0.0)
        (switch `/Game/SpaceKatana/DATA/Enums/TurnStep` (`self.TurnStep`)
          (:`NewEnumerator0`
            (`self.EndTurn` 0)
            (`self.EndTurn` 1))
          (:`NewEnumerator1`
            (`self.NewTurn`)))))
    (:`then_1`
      (`self.TimeUpdated` _output_get Amount))))

(fn `SetPlayRate`
  (params (TimeRate :type "Float (double-precision)") (DilationRate :type "Float (double-precision)"))
  (set `self.PlayRate` TimeRate)
  (`GameplayStatics.SetGlobalTimeDilation` DilationRate)
  ;[1 1 1] Override the effect of dilation in this gamemode
  (set `self.CustomTimeDilation` (/ 1.0 (`GameplayStatics.GetGlobalTimeDilation`))))

(fn `UserConstructionScript`)