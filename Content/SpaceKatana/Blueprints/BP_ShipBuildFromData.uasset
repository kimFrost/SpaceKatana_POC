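; BP_ShipBuildFromData is an actor that assembles a modular ship from a data table in its construction script.
; It reads a fixed row of DATA_Ship and adds a child actor for each module, scaling its 2D position into a flat, unrotated layout.
; Module type picks the child class: square, core and corner blocks share BP_Module, while laser turrets use BP_Turret2.
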(fn `UserConstructionScript`
  (bind _returnvalue (`|GetDataTableRow` "/Game/SpaceKatana/DATA/DATA_Ship.DATA_Ship" "NewRow")
    (:`then`
      (for _array_element (`.Modules` (break `ST_Ship` _returnvalue))
        (bind (_title _type _rotation _position) (break `ST_ShipModule` _array_element))
        (bind _returnvalue_2 (`AddComponent|Child Actor Component_0` :`RelativeTransform` (`KismetMathLibrary.MakeTransform` (`KismetMathLibrary.Conv_Vector2DToVector` (* _position 100.0)))))
        (switch `EShipModuleType` _type
          (:`BlockSquare`
            (`ChildActorComponent.SetChildActorClass` _returnvalue_2 "/Game/SpaceKatana/Blueprints/BP_Module.BP_Module_C" :!label _label))
          (:`BlockCore`
            (goto _label))
          (:`BlockCorner`
            (goto _label))
          (:`TurretLaser`
            (`ChildActorComponent.SetChildActorClass` _returnvalue_2 "/Game/SpaceKatana/Blueprints/BP_Turret2.BP_Turret2_C")))))))