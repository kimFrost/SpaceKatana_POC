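; Actor that visualizes a pending spawn-module order in Space Katana, mostly through debug drawing.
; Each Tick it casts Order to OrderSpawnModule, then draws the turns left and a fly-in direction arrow at its location.
; A valid attach hit or collision danger adds an orange or red line to the traced target and moves the SplineMesh end there.
; BeginPlay only casts; initial spline setup is disconnected.
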(event `self.ReceiveBeginPlay`
  (bind _order (`self.Order`))
  (`/Engine/EditorBlueprintResources/StandardMacros.IsValid` _order
    (:`Is Valid`
      (bind _asorder_spawn_module (cast `OrderSpawnModule` _order)))))

(event `self.ReceiveTick`
  (params (DeltaSeconds :type "Float (single-precision)"))
  (bind _returnvalue (`self.K2_GetActorLocation`))
  (bind _returnvalue_2 (`self.K2_GetActorLocation`))
  (bind _order (`self.Order`))
  (`/Engine/EditorBlueprintResources/StandardMacros.IsValid` _order
    (:`Is Valid`
      (bind _asorder_spawn_module (cast `OrderSpawnModule` _order))
      (`KismetSystemLibrary.DrawDebugString` _returnvalue (`KismetStringLibrary.Conv_IntToString` (`Order.TurnsLeft` _asorder_spawn_module)))
      (`KismetSystemLibrary.DrawDebugArrow` _returnvalue (+ (* (`OrderSpawnModule.FlyInDirection` _asorder_spawn_module) 100.0) _returnvalue) 5.0 (struct :`R` 1.0 :`B` 0.797491 :`A` 1.0) 0.0 5.0)
      (if (`OrderSpawnModule.bValidAttachHit` _asorder_spawn_module)
        (bind _tracedtargetlocation (`OrderSpawnModule.TracedTargetLocation` _asorder_spawn_module))
        (`KismetSystemLibrary.DrawDebugLine` _returnvalue_2 _tracedtargetlocation (struct :`R` 1.0 :`G` 0.633862 :`A` 1.0) 0.0 5.0)
        (`SplineMeshComponent.SetEndPosition` (`self.SplineMesh`) (- _tracedtargetlocation (`self.K2_GetActorLocation`)) true :!label _label)
        (elif (`OrderSpawnModule.bModuleCollisionDanger` _asorder_spawn_module)
          (`KismetSystemLibrary.DrawDebugLine` _returnvalue_2 _tracedtargetlocation (struct :`R` 1.0 :`G` 0.022033 :`A` 1.0) 0.0 5.0)
          (goto _label))))))

(fn `UserConstructionScript`)