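; Player or AI ship for a turn-based space battle, assembled at BeginPlay from DATA_Ship as attached block, turret and engine modules.
; GM_SpaceBattle turn events drive it: turn end moves it or fires primed turrets by mode, new turn adds power and heals the X-axis leader.
; Setting a destination costs power and is clamped by line traces against a procedural movement-field disc, dented near other ships.
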(event `FireCannons`
  (for _array_element (`self.GetAllChildActors` true)
    (bind _asbp_turret (cast `/Game/SpaceKatana/Blueprints/Modules/BP_Turret` _array_element))
    (if (`/Game/SpaceKatana/Blueprints/Modules/BP_Turret.Primed` _asbp_turret)
      (`/Game/SpaceKatana/Blueprints/Modules/BP_Turret.Fire` _asbp_turret))))

(event `MoveShip`
  (if (`self.DestinationSet`)
    (bind _asgm_space_battle (cast `/Game/SpaceKatana/Blueprints/GM_SpaceBattle` (`GameplayStatics.GetGameMode`)))
    (`KismetSystemLibrary.MoveComponentTo` (`self.K2_GetRootComponent`) (`self.ClampedDestination`) (`self.K2_GetActorRotation`) false false (`/Game/SpaceKatana/Blueprints/GM_SpaceBattle.PlayingLength` _asgm_space_battle))
    (set `self.DestinationSet` false)))

(event `self.ReceiveBeginPlay`
  (`|ExecutionSequence`
    (:`then_1`
      (bind _asgm_space_battle (cast `/Game/SpaceKatana/Blueprints/GM_SpaceBattle` (`GameplayStatics.GetGameMode`)))
      (add `/Game/SpaceKatana/Blueprints/GM_SpaceBattle.OnEndTurn` _asgm_space_battle (delegate `CustomEvent_1`))
      (add `/Game/SpaceKatana/Blueprints/GM_SpaceBattle.OnNewTurn` _asgm_space_battle (delegate `CustomEvent_0`)))
    (:`then_2`
      ;[1 1 1] Set HP to MaxHp
      (set `self.HP` (`self.MaxHP`)))
    (:`then_3`
      (`self.ConstructShip`)
      (`self.UpdateMovementField`)
      (`self.UpdateModules`))))

(event `CustomEvent_1`
  (switch `/Game/SpaceKatana/DATA/Enums/ShipMode` (`self.Mode`)
    (:`NewEnumerator0`
      (`self.MoveShip`))
    (:`NewEnumerator1`
      (`self.FireCannons`))))

(event `CustomEvent_0`
  (`self.UpdateModules`)
  (`self.UpdateMovementField`)
  (`self.AddPower` 3.0)
  (set `self.HideUI` false)
  (bind _inlead (`self.CheckInLead`))
  (if _inlead
    (`self.Heal` 1.0)))

(event `self.ReceiveTick`
  (params (DeltaSeconds :type "Float (single-precision)"))
  (bind _returnvalue (`self.K2_GetActorLocation`))
  (bind _movementfieldmesh (`self.MovementFieldMesh`))
  (if (`self.HideUI`)
    (`SceneComponent.SetHiddenInGame` _movementfieldmesh true false)
    (else
      (`SceneComponent.SetHiddenInGame` _movementfieldmesh false false)
      (`|ExecutionSequence`
        (:`then_0`
          (`KismetSystemLibrary.DrawDebugCylinder` _returnvalue _returnvalue (`self.MaxTravelDistance`) 32 (struct :`R` 1.0 :`G` 1.0 :`B` 1.0 :`A` 1.0) 0.0 2.0))
        (:`then_1`
          (if (and (`self.DestinationSet`) (`|EnumEquality` (`self.Mode`) "NewEnumerator0"))
            (`KismetSystemLibrary.DrawDebugArrow` (`self.K2_GetActorLocation`) (`self.ClampedDestination`) 50.0 (struct :`R` 0.174389 :`G` 1.0 :`A` 1.0) 0.0 2.0)))
        (:`then_2`
          (for _array_element (`self.Modules`)
            (`/Engine/EditorBlueprintResources/StandardMacros.IsValid` _array_element
              (:`Is Valid`
                (bind _returnvalue_2 (`self.K2_GetActorLocation` _array_element))
                (`KismetSystemLibrary.DrawDebugLine` (+ _returnvalue_2 (0.0 0.0 120.0)) _returnvalue_2 (struct :`R` 1.0 :`G` 0.57707 :`A` 1.0) 0.0 75.0)))))))))

(fn `AddPower`
  (params (Amount :type "Float (double-precision)"))
  (set `self.Power` (`KismetMathLibrary.FClamp` (+ (`self.Power`) Amount) 0.0 (`self.MaxPower`))))

(fn `CheckInLead`
  (returns (InLead :type Boolean))
  (bind _outactors (`GameplayStatics.GetAllActorsOfClass` "BP_Ship_C"))
  (for _array_element _outactors
    (if (!= _array_element self)
      (if (> (.x (`self.K2_GetActorLocation`)) (.x (`self.K2_GetActorLocation` _array_element)))
        (set `self.InLead` true)
        (else
          (set `self.InLead` false)
          (break)))))
  (return (`self.InLead`)))

(fn `ConstructShip`
  (locals (_ConstructModuleClass :type "/Game/SpaceKatana/Blueprints/BP_Module Class Reference" :default "/Game/SpaceKatana/Blueprints/Modules/BP_BlockSquare.BP_BlockSquare_C") (_ConstructModulesIsRoot :type Boolean))
  (`|ExecutionSequence`
    (:`then_0`
      ;[1 1 1] Core/Root
      (bind _returnvalue (`|SpawnActorFromClass` "/Game/SpaceKatana/Blueprints/Modules/BP_BlockSquare.BP_BlockSquare_C" (`KismetMathLibrary.MakeTransform` (0.0 0.0 0.0)) "AlwaysSpawn" "OverrideRootScale"))
      (bind _asbp_module (cast `/Game/SpaceKatana/Blueprints/BP_Module` _returnvalue))
      (set `ShipModule.bIsRoot` true _asbp_module)
      (`self.K2_AttachToActor` _returnvalue self "None" "KeepRelative" "SnapToTarget" "SnapToTarget" true)
      (set `self.RootModule` _asbp_module))
    (:`then_1`
      (bind _returnvalue_2 (`|GetDataTableRow` "/Game/SpaceKatana/DATA/DATA_Ship.DATA_Ship" "NewRow")
        (:`then`
          (for _array_element (`.Modules` (break `ST_Ship` _returnvalue_2))
            (bind (_title _type _rotation _position) (break `ST_ShipModule` _array_element))
            (switch `EShipModuleType` _type
              (:`BlockSquare`
                (set `local._ConstructModuleClass` "/Game/SpaceKatana/Blueprints/Modules/BP_BlockSquare.BP_BlockSquare_C" :!label _label))
              (:`BlockCorner`
                (goto _label))
              (:`TurretLaser`
                (set `local._ConstructModuleClass` "/Game/SpaceKatana/Blueprints/Modules/BP_Turret.BP_Turret_C"))
              (:`Engine`
                (set `local._ConstructModuleClass` "/Game/SpaceKatana/Blueprints/Modules/BP_Engine.BP_Engine_C")))
            (bind _returnvalue_3 (`|SpawnActorFromClass` (`local._ConstructModuleClass`) (`KismetMathLibrary.MakeTransform` (`KismetMathLibrary.Conv_Vector2DToVector` (* _position 100.0)) (`KismetMathLibrary.MakeRotator` 0.0 0.0 _rotation) (1.0 1.0 1.0)) "AlwaysSpawn" "OverrideRootScale"))
            (cast `/Game/SpaceKatana/Blueprints/BP_Module` _returnvalue_3)
            (`self.K2_AttachToActor` _returnvalue_3 self "None" "KeepRelative" "KeepRelative" "KeepRelative" true)))))))

(fn `DrainPower`
  (params (Amount :type "Float (double-precision)"))
  (returns (Drained :type Boolean))
  (bind _returnvalue (- (`self.Power`) Amount))
  (if (>= _returnvalue 0.0)
    (set `self.Power` _returnvalue)
    (return true)
    (else
      (return false))))

(fn `GetClosestValidMoveLocation`
  (params (Location :type "Vector Structure"))
  (returns (ValidMoveLocation :type "Vector Structure"))
  (bind _returnvalue (`self.K2_GetActorLocation`))
  (bind _returnvalue_2 (`KismetMathLibrary.FCeil` (/ (`KismetMathLibrary.VSize` (- Location (`self.K2_GetActorLocation`))) 10.0)))
  (bind (_hitlocation _hitnormal _bonename _returnvalue_3) (`PrimitiveComponent.K2_LineTraceComponent` (`self.MovementFieldMesh`) (+ Location (0.0 0.0 500.0)) (+ Location (0.0 0.0 -500.0)) true false))
  (if _returnvalue_3
    (return Location)
    (else
      (for _index (range (+ _returnvalue_2 1))
        (bind _returnvalue_4 (+ _returnvalue (* (`KismetMathLibrary.Normal` (- Location _returnvalue)) (* (- _returnvalue_2 _index) 10))))
        (bind (_hitlocation_2 _hitnormal_2 _bonename_2 _returnvalue_5) (`PrimitiveComponent.K2_LineTraceComponent` (`self.MovementFieldMesh`) (+ _returnvalue_4 (0.0 0.0 100.0)) (+ _returnvalue_4 (0.0 0.0 -100.0)) true false))
        (if _returnvalue_5
          (return _hitlocation_2)))
      (return (0.0 0.0 0.0)))))

(fn `Heal`
  (params (Amount :type "Float (double-precision)"))
  (set `self.HP` (`KismetMathLibrary.FClamp` (+ (`self.HP`) Amount) 0.0 (`self.MaxHP`))))

(fn `ResetTravel`
  (if (`self.DestinationSet`)
    (set `self.DestinationSet` false)
    (`self.AddPower` (`self.TravelPowerCost`))))

(fn `SetDestination`
  (params (Location :type "Vector Structure"))
  (bind _output_get (set `self.Destination` (`KismetMathLibrary.MakeVector` (.x Location) (.y Location))))
  (set `self.DestinationRelative` (- _output_get (`self.K2_GetActorLocation`)))
  (if (not (`self.DestinationSet`))
    (bind _drained (`self.DrainPower` (`self.TravelPowerCost`)))
    (set `self.DestinationSet` _drained))
  (bind _validmovelocation (`self.GetClosestValidMoveLocation` (`self.Destination`)))
  (set `self.ClampedDestination` (`KismetMathLibrary.MakeVector` (.x _validmovelocation) (.y _validmovelocation))))

(fn `TakeDamge`
  (params (Amount :type "Float (double-precision)"))
  (set `self.HP` (- (`self.HP`) Amount)))

(fn `UpdateMovementField`
  (locals (_Verticies :type "Array of Vector Structure") (_Triangles :type "Array of Integer") (_Normals :type "Array of Vector Structure") (_UVs :type "Array of Vector2D Structure"))
  (bind __triangles (`local._Triangles`))
  (bind __triangles_2 (`local._Triangles`))
  (bind _maxtraveldistance (`self.MaxTravelDistance`))
  (bind _movementfieldmesh (`self.MovementFieldMesh`))
  (bind _returnvalue (`KismetArrayLibrary.Array_LastIndex` (`local._Verticies`)))
  (`|ExecutionSequence`
    (:`then_0`
      (`KismetArrayLibrary.Array_Clear` (`local._Verticies`))
      (`KismetArrayLibrary.Array_Clear` (`local._Triangles`))
      ;[1 1 1] Center vertice
      (`KismetArrayLibrary.Array_Add` (`local._Verticies`) (0.0 0.0 0.0))
      (for _index (range 201)
        (`KismetArrayLibrary.Array_Add` (`local._Verticies`) (`KismetMathLibrary.RotateAngleAxis` (`KismetMathLibrary.MakeVector` (`self.MaxTravelDistance`)) (* _index (/ 360.0 200.0)) (0.0 0.0 1.0)))
        (if (> _index 0)
          (`KismetArrayLibrary.Array_Add` __triangles)
          (`KismetArrayLibrary.Array_Add` __triangles _index)
          (`KismetArrayLibrary.Array_Add` __triangles (- _index 1))))
      (`KismetArrayLibrary.Array_Add` __triangles_2)
      (`KismetArrayLibrary.Array_Add` __triangles_2 _returnvalue)
      (`KismetArrayLibrary.Array_Add` __triangles_2 (- _returnvalue 1)))
    (:`then_1`
      (bind _outactors (`GameplayStatics.GetAllActorsOfClass` "BP_Ship_C"))
      (for _array_element _outactors
        (if (!= _array_element self)
          (for (_array_element_2 _array_index) (`local._Verticies`)
            (bind _returnvalue_2 (`KismetMathLibrary.VSize` (- (`self.K2_GetActorLocation` _array_element) (+ _array_element_2 (`self.K2_GetActorLocation` self)))))
            (if (< _returnvalue_2 _maxtraveldistance)
              (`KismetArrayLibrary.Array_Set` (`local._Verticies`) _array_index (* _array_element_2 (/ _returnvalue_2 _maxtraveldistance))))))))
    (:`then_2`
      (`ProceduralMeshComponent.ClearAllMeshSections` _movementfieldmesh)
      (`ProceduralMeshComponent.CreateMeshSection_LinearColor` :`self` _movementfieldmesh :`Vertices` (`local._Verticies`) :`Triangles` (`local._Triangles`) :`Normals` (`local._Normals`) :`UV0` (`local._UVs`) :`bCreateCollision` true)
      (`PrimitiveComponent.SetMaterial` (`self.MovementFieldMesh`) 0 "/Game/SpaceKatana/Materials/M_MovementField.M_MovementField"))))

(fn `UserConstructionScript`)