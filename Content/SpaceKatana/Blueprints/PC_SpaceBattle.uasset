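; Player controller for the space battle that lets the player queue module spawn orders on a grid during the Planning step.
; Tick projects the cursor onto a horizontal plane and draws a debug arrow along the spawn direction, which R rotates by 90 degrees.
; Left click offsets that point back to the row or column edge and sends a block order to GM_SpaceBattle; right click reverts to Select.
; Older ship and turret controls remain as disconnected code.
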(event `self.ReceiveTick`
  (params (DeltaSeconds :type "Float (single-precision)"))
  (bind (_worldlocation _worlddirection) (`self.DeprojectMousePositionToWorld`))
  (bind (_t _intersection) (`KismetMathLibrary.LinePlaneIntersection_OriginNormal` _worldlocation (+ _worldlocation (* _worlddirection 10000.0)) (0.0 0.0 0.0) (0.0 0.0 1.0)))
  (`KismetSystemLibrary.DrawDebugArrow` _intersection (+ _intersection (* (`self.SpawnInDirection`) 100.0)) 100.0 (struct :`G` 0.032635 :`B` 1.0 :`A` 1.0) 0.0 5.0))

(event `Key|LeftMouseButton`
  (params (Key :type "Key Structure" :default "AnyKey"))
  (bind (_worldlocation _worlddirection) (`self.DeprojectMousePositionToWorld`))
  (:`Pressed`
    (switch `EToolType` (`self.CurrentTool`)
      (:`SpawnModule`
        (bind _asgm_space_battle (cast `/Game/SpaceKatana/Blueprints/GM_SpaceBattle` (`GameplayStatics.GetGameMode`)))
        (switch `ETurnStep` (`GameModeBattle.CurrentStep` _asgm_space_battle)
          (:`Planning`
            (bind _returnvalue (`GameModeBattle.WorldLocationToCoords` _asgm_space_battle (- (`.Intersection` (`KismetMathLibrary.LinePlaneIntersection_OriginNormal` _worldlocation (+ _worldlocation (* _worlddirection 10000.0)) (0.0 0.0 0.0) (0.0 0.0 1.0))) (* (`self.SpawnInDirection`) 25000.0)) true))
            (bind (_x _y) (`KismetMathLibrary.BreakVector2D` _returnvalue))
            (`GameModeBattle.AddOrder_SpawnModule` _asgm_space_battle "/Game/SpaceKatana/Blueprints/Modules/BP_BlockSquare.BP_BlockSquare_C" (`KismetMathLibrary.FTrunc` _x) (`KismetMathLibrary.FTrunc` _y) (`self.SpawnInDirection`) null)))))))

(event `Key|R`
  (params (Key :type "Key Structure" :default "AnyKey"))
  (:`Pressed`
    (`self.RotateDirection`)))

(event `Key|RightMouseButton`
  (params (Key :type "Key Structure" :default "AnyKey"))
  (:`Pressed`
    ;[1 1 1] Cancel Current Tool
    (set `self.CurrentTool` "Select")))

(fn `RotateDirection`
  (set `self.SpawnInDirection` (`KismetMathLibrary.RotateAngleAxis` (`self.SpawnInDirection`) 90.0 (0.0 0.0 1.0))))

(fn `UserConstructionScript`)